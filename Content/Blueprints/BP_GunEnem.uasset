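; BP_GunEnem is a flipbook-sprite enemy that flees from the player and never attacks in this graph.
; BeginPlay loads sprites and key info from DT_Enemy by TypeName.
; Entering RunRadius starts repeated AIMoveTo hops away from the player with random yaw spread; leaving starts a timer back to spawn.
; Tick selects idle or walk sprites by HP and velocity, and at zero HP shows Scientist_Dead, then destroys the actor.
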(event OnComponentBeginOverlap(RunRadius)
  (params (OverlappedComponent :type Primitive%20Component%20Object%20Reference) (OtherActor :type Actor%20Object%20Reference) (OtherComp :type Primitive%20Component%20Object%20Reference) (OtherBodyIndex :type Integer) (bFromSweep :type Boolean) (SweepResult :type Hit%20Result%20Structure%20%28by%20ref%29))
  (Utilities|Casting|CastToBP_ThirdPersonCharacter OtherActor)
  (Variables|Default|SetIsRunning true)
  (Utilities|Time|ClearTimerbyFunctionName 0 "ReturnToSpawn")
  (CallFunction|RunAway))

(event OnComponentEndOverlap(RunRadius)
  (params (OverlappedComponent :type Primitive%20Component%20Object%20Reference) (OtherActor :type Actor%20Object%20Reference) (OtherComp :type Primitive%20Component%20Object%20Reference) (OtherBodyIndex :type Integer))
  (Utilities|Casting|CastToBP_ThirdPersonCharacter OtherActor)
  (Variables|Default|SetIsRunning false)
  (Utilities|Time|SetTimerbyFunctionName 0 "ReturnToSpawn" 1e+01))

(event Custom|RunAway
  (bind _returnvalue (Math|Random|RandomFloatinRange -3e+01 3e+01))
  (bind _returnvalue_2 (Transformation|GetActorLocation))
  (bind _bp_third_person_character (Variables|Default|GetBP%20Third%20Person%20Character))
  (bind _returnvalue_3 (Transformation|GetActorLocation _bp_third_person_character))
  (bind _returnvalue_4 (Math|Rotator|FindLookatRotation _returnvalue_2 _returnvalue_3))
  (bind _returnvalue_5 (+ (.yaw _returnvalue_4) _returnvalue))
  (bind _returnvalue_6 (Math|Vector|GetForwardVector (Math|Rotator|MakeRotator 0.0 0.0 _returnvalue_5)))
  (bind _returnvalue_7 (* _returnvalue_6 -1e+02))
  (bind _returnvalue_8 (+ _returnvalue_2 _returnvalue_7))
  (bind (_x _y) (Math|Vector|BreakVector _returnvalue_8))
  (AI|AIMoveTo self (Math|Vector|MakeVector _x _y 0.0) 0 5.0 false
    (:OnSuccess
      _)
    (:OnFail
      _))
  (if (Variables|Default|GetIsRunning)
    (CallFunction|RunAway)))

(event EventBeginPlay
  (bind _asbp_third_person_character (Utilities|Casting|CastToBP_ThirdPersonCharacter (Game|GetPlayerCharacter 0)))
  (Variables|Default|SetBP%20Third%20Person%20Character _asbp_third_person_character)
  (Variables|Default|SetStartLocation (Transformation|GetWorldLocation (Variables|Collision|GetCapsuleComponent)))
  (bind _returnvalue (Utilities|GetDataTableRow "/Game/Blueprints/DT_Enemy.DT_Enemy" (Variables|Default|GetTypeName))
    (:then
      (Variables|Default|SetSprite%20Idle (.Sprite_Idle (Utilities|Struct|BreakS_EnemyType _returnvalue)))
      (Variables|Default|SetSprite%20Idle%20Hurt%201 (.Sprite_Idle_Hurt1 (Utilities|Struct|BreakS_EnemyType _returnvalue)))
      (Variables|Default|SetSprite%20Idle%20Hurt%202 (.Sprite_Idle_Hurt2 (Utilities|Struct|BreakS_EnemyType _returnvalue)))
      (Variables|Default|SetSprite%20Walk (.Sprite_Walk (Utilities|Struct|BreakS_EnemyType _returnvalue)))
      (Variables|Default|SetSprite%20Walk%20Hurt%201 (.Sprite_Walk_Hurt1 (Utilities|Struct|BreakS_EnemyType _returnvalue)))
      (Variables|Default|SetSprite%20Walk%20Hurt%202 (.Sprite_Walk_Hurt2 (Utilities|Struct|BreakS_EnemyType _returnvalue)))
      (Variables|Default|SetHas%20Key (.HasKey (Utilities|Struct|BreakS_EnemyType _returnvalue)))
      (Variables|Default|SetKey%20Color (.KeyColor (Utilities|Struct|BreakS_EnemyType _returnvalue))))))

(event EventTick
  (params (DeltaSeconds :type Float%20%28single-precision%29))
  (bind _returnvalue (Transformation|GetVelocity))
  (bind _enemyhp (Variables|Default|GetEnemyHP))
  (bind _scientistflipbook (Variables|Default|GetScientistFlipbook))
  (bind _enemyhp_2 (Variables|Default|GetEnemyHP))
  (bind _scientistflipbook_2 (Variables|Default|GetScientistFlipbook))
  (Transformation|SetWorldRotation (Variables|Default|GetScene) "0, 0, 0" false false)
  (if (> (Variables|Default|GetEnemyHP) 0)
    (if (or (> (.x _returnvalue) 0.0) (> (.y _returnvalue) 0.0))
      ;[0.15 0.15 0.15 0.5] Running Sprite Logic
      (if (== _enemyhp 3)
        (Sprite|SetFlipbook _scientistflipbook (Variables|Default|GetSprite%20Walk))
        (elif (== _enemyhp 2)
          (Sprite|SetFlipbook _scientistflipbook (Variables|Default|GetSprite%20Walk%20Hurt%201))
          (else
            (Sprite|SetFlipbook _scientistflipbook (Variables|Default|GetSprite%20Walk%20Hurt%202)))))
      (else
        ;[0.15 0.15 0.15 0.5] Idle Sprite Logic
        (if (== _enemyhp_2 3)
          (Sprite|SetFlipbook _scientistflipbook_2 (Variables|Default|GetSprite%20Idle))
          (elif (== _enemyhp_2 2)
            (Sprite|SetFlipbook _scientistflipbook_2 (Variables|Default|GetSprite%20Idle%20Hurt%201))
            (else
              (Sprite|SetFlipbook _scientistflipbook_2 (Variables|Default|GetSprite%20Idle%20Hurt%202)))))))
    (else
      (Variables|/Script/Engine.CharacterMovementComponent|SetMaxWalkSpeed (Variables|Character|GetCharacterMovement) 0.0)
      (Sprite|SetFlipbook (Variables|Default|GetScientistFlipbook) "/Game/Sprites/Scientist/Scientist_Dead.Scientist_Dead")
      (Utilities|FlowControl|Delay 5.0)
      (Actor|DestroyActor))))

(fn ConstructionScript)

(fn ReturntoSpawn
  (AI|Navigation|SimpleMovetoLocation (Pawn|GetController) (Variables|Default|GetStartLocation)))