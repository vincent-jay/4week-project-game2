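; BP_BaseEnem is a 2D flipbook scientist enemy that flees the player while they are inside its RunRadius.
; RunAway repeats short AI moves away from the player with random yaw spread, retrying on success or failure while IsRunning.
; Tick locks the Scene component's world rotation and picks idle or walk flipbooks by EnemyHP.
; At zero HP it zeroes walk speed, shows the dead sprite and destroys itself after a delay.
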(event OnComponentBeginOverlap(RunRadius)
  (params (OverlappedComponent :type Primitive%20Component%20Object%20Reference) (OtherActor :type Actor%20Object%20Reference) (OtherComp :type Primitive%20Component%20Object%20Reference) (OtherBodyIndex :type Integer) (bFromSweep :type Boolean) (SweepResult :type Hit%20Result%20Structure%20%28by%20ref%29))
  (Utilities|Casting|CastToBP_ThirdPersonCharacter OtherActor)
  (Variables|Default|SetIsRunning true)
  (CallFunction|RunAway))

(event OnComponentEndOverlap(RunRadius)
  (params (OverlappedComponent :type Primitive%20Component%20Object%20Reference) (OtherActor :type Actor%20Object%20Reference) (OtherComp :type Primitive%20Component%20Object%20Reference) (OtherBodyIndex :type Integer))
  (Utilities|Casting|CastToBP_ThirdPersonCharacter OtherActor)
  (Variables|Default|SetIsRunning false))

(event Custom|RunAway
  (bind _returnvalue (Math|Random|RandomFloatinRange -3e+01 3e+01))
  (bind _returnvalue_2 (Transformation|GetActorLocation))
  (bind _bp_third_person_character (Variables|Default|GetBP%20Third%20Person%20Character))
  (bind _returnvalue_3 (Transformation|GetActorLocation _bp_third_person_character))
  (bind _returnvalue_4 (Math|Rotator|FindLookatRotation _returnvalue_2 _returnvalue_3))
  (bind _returnvalue_5 (+ (.yaw _returnvalue_4) _returnvalue))
  (bind _returnvalue_6 (Math|Vector|GetForwardVector (Math|Rotator|MakeRotator 0.0 0.0 _returnvalue_5)))
  (bind _returnvalue_7 (* _returnvalue_6 -1e+02))
  (bind _returnvalue_8 (+ _returnvalue_2 _returnvalue_7))
  (bind (_x _y) (Math|Vector|BreakVector _returnvalue_8))
  (AI|AIMoveTo self (Math|Vector|MakeVector _x _y 0.0) 0 5.0 false
    (:OnSuccess
      _)
    (:OnFail
      _))
  (if (Variables|Default|GetIsRunning)
    (CallFunction|RunAway)))

(event EventBeginPlay
  (bind _asbp_third_person_character (Utilities|Casting|CastToBP_ThirdPersonCharacter (Game|GetPlayerCharacter 0)))
  (Variables|Default|SetBP%20Third%20Person%20Character _asbp_third_person_character))

(event EventTick
  (params (DeltaSeconds :type Float%20%28single-precision%29))
  (bind _enemyhp (Variables|Default|GetEnemyHP))
  (bind _scientistflipbook (Variables|Default|GetScientistFlipbook))
  (bind _enemyhp_2 (Variables|Default|GetEnemyHP))
  (bind _scientistflipbook_2 (Variables|Default|GetScientistFlipbook))
  (Transformation|SetWorldRotation (Variables|Default|GetScene) "0.000000,0.000000,0.000000" false false)
  (if (> (Variables|Default|GetEnemyHP) 0)
    (if (Variables|Default|GetIsRunning)
      ;[0.15 0.15 0.15 0.5] Running Sprite Logic
      (if (== _enemyhp 3)
        (Sprite|SetFlipbook _scientistflipbook "/Game/Sprites/Scientist/Scientist_Walk.Scientist_Walk")
        (elif (== _enemyhp 2)
          (Sprite|SetFlipbook _scientistflipbook "/Game/Sprites/Scientist/Scientist_Hurt2_Walk.Scientist_Hurt2_Walk")
          (else
            (Sprite|SetFlipbook _scientistflipbook "/Game/Sprites/Scientist/Scientist_Hurt3_Walk.Scientist_Hurt3_Walk"))))
      (else
        ;[0.15 0.15 0.15 0.5] Idle Sprite Logic
        (if (== _enemyhp_2 3)
          (Sprite|SetFlipbook _scientistflipbook_2 "/Game/Sprites/Scientist/Scientist_Idle.Scientist_Idle")
          (elif (== _enemyhp_2 2)
            (Sprite|SetFlipbook _scientistflipbook_2 "/Game/Sprites/Scientist/Scientist_Hurt2_Idle.Scientist_Hurt2_Idle")
            (else
              (Sprite|SetFlipbook _scientistflipbook_2 "/Game/Sprites/Scientist/Scientist_Hurt3_Idle.Scientist_Hurt3_Idle"))))))
    (else
      (Variables|/Script/Engine.CharacterMovementComponent|SetMaxWalkSpeed (Variables|Character|GetCharacterMovement) 0.0)
      (Sprite|SetFlipbook (Variables|Default|GetScientistFlipbook) "/Game/Sprites/Scientist/Scientist_Dead.Scientist_Dead")
      (Utilities|FlowControl|Delay 5.0)
      (Actor|DestroyActor))))

(fn ConstructionScript)